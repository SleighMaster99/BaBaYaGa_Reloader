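; BP_EnemyController is the enemy AI controller, which runs BT_EnemyBehaviorTree on BeginPlay.
; Its PawnSensing hearing event writes heard noise locations into the blackboard for the behavior tree.
; A DistanceToPlayer check compares its own location with BP_Player's against a given distance, clearing the noise location when the player is not within range.
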(event OnHearNoise(PawnSensing)
  (params (Instigator :type Pawn%20Object%20Reference) (Location :type Vector%20%28by%20ref%29 :default "0, 0, 0") (Volume :type Float%20%28single-precision%29))
  (AI|Components|Blackboard|SetValueasVector (AI|GetBlackboard 0) (Variables|Default|GetNoiseVectorKeyName) Location))

(event EventBeginPlay
  (AI|RunBehaviorTree "/Game/Enemy/BT_EnemyBehaviorTree.BT_EnemyBehaviorTree"))

(fn ConstructionScript)

(fn DistancetoPlayer
  (params (Distance :type Float%20%28double-precision%29))
  (bind _asbp_player (Utilities|Casting|CastToBP_Player (Game|GetPlayerCharacter 0)))
  (if (< (Math|Vector|Distance(Vector) (Transformation|GetActorLocation _asbp_player) (Transformation|GetActorLocation self)) Distance)
    (return true)
    (else
      (AI|Components|Blackboard|ClearValue (AI|GetBlackboard 0) (Variables|Default|GetNoiseVectorKeyName))
      (return false))))